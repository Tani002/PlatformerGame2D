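; NPC Blueprint that shows an interaction prompt and steps through lines of dialogue with the player.
; Box overlap toggles the text render and Player_BP's TriggerButton, and creates or removes a DialogueInterface widget.
; EventDialogueOccurs passes NPCText to the widget, reveals it, and advances its Textrow, removing the widget at the last line.
; A DoOnce gates each step and is reset afterwards.
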(event OnComponentBeginOverlap(Box)
  (params (OverlappedComponent :type Primitive%20Component%20Object%20Reference) (OtherActor :type Actor%20Object%20Reference) (OtherComp :type Primitive%20Component%20Object%20Reference) (OtherBodyIndex :type Integer) (bFromSweep :type Boolean) (SweepResult :type Hit%20Result%20Structure%20%28by%20ref%29))
  ;[1 1 1] Text Interact and Talk Button POP-UP on Collision Trigger
  (bind _asplayer_bp (Utilities|Casting|CastToPlayer_BP OtherActor))
  (Development|SetHiddeninGame (Variables|Default|GetTextRender) false false)
  (Variables|/Game/Blueprints/Player_BP.Player_BP_C|SetTriggerButton _asplayer_bp true)
  (bind _returnvalue (UserInterface|CreateWidget "/Game/UserInterface/DialogueInterface.DialogueInterface_C"))
  (bind _output_get (Variables|Default|SetDialogueUI _returnvalue))
  (UserInterface|Viewport|AddtoViewport _output_get 0))

(event OnComponentEndOverlap(Box)
  (params (OverlappedComponent :type Primitive%20Component%20Object%20Reference) (OtherActor :type Actor%20Object%20Reference) (OtherComp :type Primitive%20Component%20Object%20Reference) (OtherBodyIndex :type Integer))
  (bind _dialogueui (Variables|Default|GetDialogueUI))
  ;[1 1 1] Text Interact and Talk Button POP-UP on Collision Trigger
  (bind _asplayer_bp (Utilities|Casting|CastToPlayer_BP OtherActor))
  (Development|SetHiddeninGame (Variables|Default|GetTextRender) true false)
  (Variables|/Game/Blueprints/Player_BP.Player_BP_C|SetTriggerButton _asplayer_bp false)
  (Utilities|IsValid _dialogueui
    (:Is%20Valid
      (Widget|RemovefromParent _dialogueui))))

(event Custom|resetDialogue
  ;[1 1 1] Dialogue System That Checks Every Element For Every Dialogue Then Destroys It After Reaching The Maximum Value
  (Utilities|FlowControl|DoOnce false) ; enters at Reset
)

(event EventBeginPlay)

(event EventTick
  (params (DeltaSeconds :type Float%20%28single-precision%29)))

(event EventEventDialogueOccurs
  ;[1 1 1] Dialogue System That Checks Every Element For Every Dialogue Then Destroys It After Reaching The Maximum Value
  (Utilities|FlowControl|DoOnce false
    (:Completed
      (Variables|/Game/UserInterface/DialogueInterface.DialogueInterface_C|Settext (Variables|Default|GetDialogueUI) (Variables|Default|GetNPCText))
      (Widget|SetVisibility (Variables|/Game/UserInterface/DialogueInterface.DialogueInterface_C|GetImage_0 (Variables|Default|GetDialogueUI)) "Visible")
      (if (> (+ (Variables|/Game/UserInterface/DialogueInterface.DialogueInterface_C|Gettextrow (Variables|Default|GetDialogueUI)) 1) (- (Utilities|Array|Length (Variables|Default|GetNPCText)) 1))
        (Widget|RemovefromParent (Variables|Default|GetDialogueUI))
        (CallFunction|ResetDialogue)
        (else
          (Variables|/Game/UserInterface/DialogueInterface.DialogueInterface_C|Settextrow (Variables|Default|GetDialogueUI) (+ (Variables|/Game/UserInterface/DialogueInterface.DialogueInterface_C|Gettextrow (Variables|Default|GetDialogueUI)) 1))
          (CallFunction|ResetDialogue))))))

(fn ConstructionScript)